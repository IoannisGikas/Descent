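; Base Blueprint for RPG characters that respond to interaction with a placeholder dialogue line.
; BeginPlay turns off shadow casting on the dialogue indicator and caches the GM_RPG game mode.
; Interact calls ShowDialogLine, which invokes BubblePosition on the game mode's HUD widget and returns a hardcoded greeting that is printed to screen.
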(event `self.ReceiveBeginPlay`
  (`PrimitiveComponent.SetCastShadow` (`self.DIalogueIndicator`) false)
  (bind _asgm_rpg (cast `/Game/Blueprints/GM_RPG` (`GameplayStatics.GetGameMode`)))
  (set `self.Gamemode` _asgm_rpg))

(event `/Game/Blueprints/Interfaces/BPI_Interaction.Interact`
  (bind _dialog (`self.ShowDialogLine`))
  (`KismetSystemLibrary.PrintString` _dialog))

(fn `ShowDialogLine`
  (returns (Dialog :type String))
  (`/Game/Widgets/WBP_Hud.BubblePosition` (`/Game/Blueprints/GM_RPG.HUDwiget` (`self.Gamemode`)))
  (return "Welcome"))

(fn `UserConstructionScript`)